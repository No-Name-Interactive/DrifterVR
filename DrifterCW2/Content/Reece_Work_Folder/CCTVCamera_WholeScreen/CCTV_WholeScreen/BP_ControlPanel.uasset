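; Interactable CCTV control panel that shows its security cameras on the player's whole screen.
; On interaction, if cameras exist and no one occupies it, it moves input from the player to itself and switches the view target to the first camera.
; Left and right inputs cycle through the camera array with wraparound.
; The panel interact input restores the player's view and input and frees the panel.
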(event EventOnInteraction
  (params (Player :type Vive%20Pawn%20Character%20Object%20Reference))
  (bind _returnvalue (Pawn|GetController Player))
  (bind _asplayer_controller (Utilities|Casting|CastToPlayerController _returnvalue))
  ;[1 1 1] Checks if the control panel is in use
  (if (and (Private|HasCameras?) (not (Private|Occupied?)))
    ;[1 1 1] If control panel is useable disable all input aside from specified Control Panel inputs
    (Variables|Default|SetOccupiedPlayer Player)
    (Input|DisableInput Player _asplayer_controller)
    (Input|EnableInput _asplayer_controller)
    (Variables|Default|SetActiveCameraIndex 0)
    (Private|SetViewTargetasActiveCamera)))

(event Input|ActionEvents|InputActionPanel_Interact
  (params (Key :type Key%20Structure :default "None"))
  ;[1 1 1] Once Control Panel is not in use, player gains back input controls
  (:Pressed
    (Game|Player|SetViewTargetwithBlend (.AsPlayer%20Controller (Utilities|Casting|CastToPlayerController (Pawn|GetController (Variables|Default|GetOccupiedPlayer)))) (Variables|Default|GetOccupiedPlayer) 0.0 "VTBlend_Linear" 0.0 false)
    (Input|EnableInput (Variables|Default|GetOccupiedPlayer) (.AsPlayer%20Controller (Utilities|Casting|CastToPlayerController (Pawn|GetController (Variables|Default|GetOccupiedPlayer)))))
    (Input|DisableInput (.AsPlayer%20Controller (Utilities|Casting|CastToPlayerController (Pawn|GetController (Variables|Default|GetOccupiedPlayer)))))
    (Variables|Default|SetOccupiedPlayer 0)))

(event Input|ActionEvents|InputActionSwitchCameras_R
  (params (Key :type Key%20Structure :default "None"))
  ;[1 1 1] Switches to next Camera in Order
  (:Pressed
    (Private|IncrementCameraIndex)
    (Private|SetViewTargetasActiveCamera)))

(event Input|ActionEvents|InputActionSwitchCameras_L
  (params (Key :type Key%20Structure :default "None"))
  ;[1 1 1] Switches to previous Camera in order
  (:Pressed
    (Private|DecrementCameraIndex)
    (Private|SetViewTargetasActiveCamera)))

(fn ConstructionScript)

(fn HasCameras?
  ;[1 1 1] Checks if at least 1 camera is part of the control panel
  (return (> (Utilities|Array|Length (Variables|Default|GetSecurityCameras)) 0)))

(fn Occupied?
  ;[1 1 1] Checks if Control Panel is in use
  (return (Utilities|IsValid (Variables|Default|GetOccupiedPlayer))))

(fn SetViewTargetasActiveCamera
  ;[1 1 1] Sets Active Camera
  (Game|Player|SetViewTargetwithBlend (.AsPlayer%20Controller (Utilities|Casting|CastToPlayerController (Pawn|GetController (Variables|Default|GetOccupiedPlayer)))) (Utilities|Array|Get(acopy) (Variables|Default|GetSecurityCameras) (Variables|Default|GetActiveCameraIndex)) 0.0 "VTBlend_Linear" 0.0 false))

(fn IncrementCameraIndex
  ;[1 1 1] Allows to switch to next camera in order (also loops back to the first camera after the last camera is switched)
  (if (> (+ (Variables|Default|GetActiveCameraIndex) 1) (Utilities|Array|LastIndex (Variables|Default|GetSecurityCameras)))
    (Variables|Default|SetActiveCameraIndex 0)
    (else
      (Math|Integer|IncrementInt (Variables|Default|GetActiveCameraIndex)))))

(fn DecrementCameraIndex
  ;[1 1 1] Allows to switch to Previous camera in order (also loops back to the last camera after the first camera is switched)
  (if (< (- (Variables|Default|GetActiveCameraIndex) 1) 0)
    (Variables|Default|SetActiveCameraIndex (Utilities|Array|LastIndex (Variables|Default|GetSecurityCameras)))
    (else
      (Math|Integer|DecrementInt (Variables|Default|GetActiveCameraIndex)))))