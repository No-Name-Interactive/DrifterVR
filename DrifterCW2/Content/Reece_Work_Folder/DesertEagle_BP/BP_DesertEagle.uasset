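; VR Desert Eagle pistol that the player can grip, fire and reload, with an ammo count shown on a text component.
; Its grip interface functions set single-hand gripping with physics simulation on drop, while SetHeld tracks the gripped state and holding controller.
; Shoot spawns a FirstPersonProjectile at the Arrow component when gripped with ammo left, decrementing the count.
; Moving the VRSlider to its full-progress hit point refills the ammo and refreshes the text.
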(event OnSliderHitPoint(VRSlider)
  (params (SliderProgressPoint :type Float%20%28single-precision%29))
  ;[1 1 1] Slider
  (if (== SliderProgressPoint 1.0)
    (Variables|Default|SetAmmo 7.0)
    (|SetAmmoToText_2_2)))

(event Custom|Shoot
  (bind _arrow (Variables|Default|GetArrow))
  (bind _returnvalue (Transformation|GetWorldTransform _arrow))
  ;[1 1 1] Shooting
  (if (Variables|Default|GetGripped)
    (if (> (Variables|Default|GetAmmo) 0.0)
      (Game|SpawnActorfromClass "/Game/VRExpansion/FirstPersonBP/FirstPersonBP/Blueprints/FirstPersonProjectile.FirstPersonProjectile_C" (Math|Transform|MakeTransform (.location _returnvalue) (.rotation _returnvalue) "1,1,1") "Undefined" 0 0)
      (Variables|Default|SetAmmo (- (Variables|Default|GetAmmo) 1.0))
      (|SetAmmoToText_2))))

(event Collision|EventActorBeginOverlap
  (params (OtherActor :type Actor%20Object%20Reference)))

(event EventBeginPlay
  ;[1 1 1] Ammo Text
  (|SetAmmoToText))

(event EventSetHeld
  (params (HoldingController :type Grip%20Motion%20Controller%20Component%20Object%20Reference) (GripID :type Byte :default 0) (bIsHeld :type Boolean))
  ;[1 1 1] Grip bool
  (if bIsHeld
    (Variables|Default|SetHoldingGrip (Utilities|Struct|MakeBPGripPair HoldingController GripID))
    (else
      (Variables|Default|SetHoldingGrip "")))
  (Variables|Default|SetGripped bIsHeld))

(fn ConstructionScript)

(fn AdvancedGripSettings
  (return ""))

(fn AllowsMultipleGrips
  (return false))

(fn ClosestGripSlotinRange
  (params (WorldLocation :type Vector :default "0, 0, 0") (bSecondarySlot :type Boolean) (CallingController :type Grip%20Motion%20Controller%20Component%20Object%20Reference) (OverridePrefix :type Name :default "None"))
  (return false "" "None"))

(fn DenyGripping
  (return false))

(fn GetGripScripts
  (return 0 false))

(fn GetGripStiffnessandDamping
  (return 1.5e+03 2e+02))

(fn GetPrimaryGripType
  (params (bIsSlot :type Boolean)))

(fn GripBreakDistance
  (return 1e+02))

(fn GripLateUpdateSetting
  (return "NotWhenCollidingOrDoubleGripping"))

(fn GripMovementReplicationType
  (return "ForceClientSideMovement"))

(fn IsHeld
  (return (Utilities|Array|MakeArray (Variables|Default|GetHoldingGrip)) (Variables|Default|GetGripped)))

(fn RequestsSocketing
  (return 0 "None" "" false))

(fn SecondaryGripType
  (return "SG_None"))

(fn SimulateonDrop
  (return true))

(fn TeleportBehavior
  (return "TeleportAllComponents"))