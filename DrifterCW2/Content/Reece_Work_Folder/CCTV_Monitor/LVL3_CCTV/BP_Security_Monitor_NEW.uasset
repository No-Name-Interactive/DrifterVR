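; Security monitor Blueprint that lets the player cycle its screen through nine CCTV camera feeds.
; Entering the SwitchCamera overlap volume enables input on the actor, and leaving it disables input.
; Each MonitorSecurityCameras press steps a looping MultiGate that sets the next camera material on the Screen component, starting at camera 2 and wrapping back to camera 1.
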(event OnComponentBeginOverlap(SwitchCamera)
  (params (OverlappedComponent :type Primitive%20Component%20Object%20Reference) (OtherActor :type Actor%20Object%20Reference) (OtherComp :type Primitive%20Component%20Object%20Reference) (OtherBodyIndex :type Integer) (bFromSweep :type Boolean) (SweepResult :type Hit%20Result%20Structure%20%28by%20ref%29))
  (Input|EnableInput (Game|GetPlayerController 0)))

(event OnComponentEndOverlap(SwitchCamera)
  (params (OverlappedComponent :type Primitive%20Component%20Object%20Reference) (OtherActor :type Actor%20Object%20Reference) (OtherComp :type Primitive%20Component%20Object%20Reference) (OtherBodyIndex :type Integer))
  (Input|DisableInput (Game|GetPlayerController 0)))

(event Input|ActionEvents|InputActionMonitorSecurityCameras
  (params (Key :type Key%20Structure :default "None"))
  (bind _screen (Variables|Default|GetScreen))
  (:Pressed
    (Utilities|FlowControl|MultiGate false true 0
      (:Out%200
        (Rendering|Material|SetMaterial _screen 0 "/Game/Reece_Work_Folder/CCTV_Monitor/LVL3_CCTV/Camera2/Camera2_Mat.Camera2_Mat"))
      (:Out%201
        (Rendering|Material|SetMaterial _screen 0 "/Game/Reece_Work_Folder/CCTV_Monitor/LVL3_CCTV/Camera3/Camera3_Mat.Camera3_Mat"))
      (:Out%202
        (Rendering|Material|SetMaterial _screen 0 "/Game/Reece_Work_Folder/CCTV_Monitor/LVL3_CCTV/Camera4/Camera4_Mat.Camera4_Mat"))
      (:Out%203
        (Rendering|Material|SetMaterial _screen 0 "/Game/Reece_Work_Folder/CCTV_Monitor/LVL3_CCTV/Camera5/Camera5_Mat.Camera5_Mat"))
      (:Out%204
        (Rendering|Material|SetMaterial _screen 0 "/Game/Reece_Work_Folder/CCTV_Monitor/LVL3_CCTV/Camera6/Camera6_Mat.Camera6_Mat"))
      (:Out%205
        (Rendering|Material|SetMaterial _screen 0 "/Game/Reece_Work_Folder/CCTV_Monitor/LVL3_CCTV/Camera7/Camera7_Mat.Camera7_Mat"))
      (:Out%206
        (Rendering|Material|SetMaterial _screen 0 "/Game/Reece_Work_Folder/CCTV_Monitor/LVL3_CCTV/Camera8/Camera8_Mat.Camera8_Mat"))
      (:Out%207
        (Rendering|Material|SetMaterial _screen 0 "/Game/Reece_Work_Folder/CCTV_Monitor/LVL3_CCTV/Camera9/Camera9_Mat.Camera9_Mat"))
      (:Out%208
        (Rendering|Material|SetMaterial _screen 0 "/Game/Reece_Work_Folder/CCTV_Monitor/LVL3_CCTV/Camera1/Camera1_Mat.Camera1_Mat")))))

(fn ConstructionScript)