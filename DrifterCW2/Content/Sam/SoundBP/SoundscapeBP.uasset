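; SoundscapeBP is an ambient noise source that registers itself with the Vive pawn and exposes a Loudness value.
; Activation overlaps add or remove it from the pawn's Soundscape while tracking Player; StartOn instead caches the pawn at BeginPlay and updates LocalSounds.
; Tick sets Loudness to Volume when Player is valid, IsOn and not Destroyed, otherwise zero, with debug printing.
; The switch and damage events are unfinished, changing no state.
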(event OnComponentBeginOverlap(Activation)
  (params (OverlappedComponent :type Primitive%20Component%20Object%20Reference) (OtherActor :type Actor%20Object%20Reference) (OtherComp :type Primitive%20Component%20Object%20Reference) (OtherBodyIndex :type Integer) (bFromSweep :type Boolean) (SweepResult :type Hit%20Result%20Structure%20%28by%20ref%29))
  ;[1 1 1] On Begin and End Overlap
  (if (Variables|Default|GetIsOn)
    (bind _asvive_pawn_character (Utilities|Casting|CastToVive_PawnCharacter OtherActor))
    (Utilities|Array|AddUnique (Variables|/Game/VRExpansion/Vive/Vive_PawnCharacter.Vive_PawnCharacter_C|GetSoundscape _asvive_pawn_character) self)
    (Variables|Default|SetPlayer _asvive_pawn_character)))

(event OnComponentEndOverlap(Activation)
  (params (OverlappedComponent :type Primitive%20Component%20Object%20Reference) (OtherActor :type Actor%20Object%20Reference) (OtherComp :type Primitive%20Component%20Object%20Reference) (OtherBodyIndex :type Integer))
  ;[1 1 1] On Begin and End Overlap
  (bind _asvive_pawn_character (Utilities|Casting|CastToVive_PawnCharacter OtherActor))
  (Utilities|Array|RemoveItem (Variables|/Game/VRExpansion/Vive/Vive_PawnCharacter.Vive_PawnCharacter_C|GetSoundscape _asvive_pawn_character) self)
  (Variables|Default|SetPlayer 0))

(event Custom|CustomEvent
  (params (Damage :type Integer))
  ;[1 1 1] On/Off
  ;;[1 1 1] Damage
  (Variables|Default|SetDestroyed (Variables|Default|GetDestroyed)))

(event Custom|CustomEvent_1
  ;[1 1 1] On/Off
  ;;[1 1 1] Switch Interface
  (bind _isa (Utilities|FlowControl|FlipFlop) ; IsOn?
    (:A
      (if (Variables|Default|GetDestroyed)
        _))))

(event EventTick
  (params (DeltaSeconds :type Float%20%28single-precision%29))
  ;[1 1 1] Ambient Noise
  (Utilities|IsValid (Variables|Default|GetPlayer)
    (:Is%20Valid
      (if (Variables|Default|GetDestroyed)
        (Variables|Default|SetLoudness 0.0 :!label _label)
        (elif (Variables|Default|GetIsOn)
          (bind _output_get (Variables|Default|SetLoudness (Variables|Default|GetVolume)))
          (Development|PrintText (Utilities|Text|FormatText "{y} loudness" _output_get) true true "(R=0.011136,G=1.000000,B=0.000000,A=1.000000)")
          (else
            (goto _label)))))
    (:Is%20Not%20Valid
      (Variables|Default|SetLoudness 0.0))))

(event EventBeginPlay
  ;[1 1 1] BeginPlay
  (if (Variables|Default|GetStartOn)
    (bind _returnvalue (Actor|GetActorOfClass "/Game/VRExpansion/Vive/Vive_PawnCharacter.Vive_PawnCharacter_C"))
    (bind _asvive_pawn_character (Utilities|Casting|CastToVive_PawnCharacter _returnvalue))
    (Utilities|Array|AddUnique (Variables|/Game/VRExpansion/Vive/Vive_PawnCharacter.Vive_PawnCharacter_C|GetLocalSounds _asvive_pawn_character) 0)
    (Variables|Default|SetPlayer _asvive_pawn_character)))

(fn ConstructionScript)