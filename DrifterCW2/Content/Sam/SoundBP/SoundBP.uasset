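; SoundBP is an ambient noise source that registers itself in a Vive pawn's LocalSounds while overlapping its sphere, if switched on at entry.
; With a player inside, Tick computes Loudness through a falloff math expression fed the audio attenuation distance, and prints the player's distance for debugging.
; Loudness drops to zero when off or destroyed.
; The damage and switch events are stubs that change no state.
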(event OnComponentBeginOverlap(Sphere)
  (params (OverlappedComponent :type Primitive%20Component%20Object%20Reference) (OtherActor :type Actor%20Object%20Reference) (OtherComp :type Primitive%20Component%20Object%20Reference) (OtherBodyIndex :type Integer) (bFromSweep :type Boolean) (SweepResult :type Hit%20Result%20Structure%20%28by%20ref%29))
  ;[1 1 1] On Begin and End Overlap
  (if (Variables|Default|GetIsOn)
    (bind _asvive_pawn_character (Utilities|Casting|CastToVive_PawnCharacter OtherActor))
    (Utilities|Array|AddUnique (Variables|/Game/VRExpansion/Vive/Vive_PawnCharacter.Vive_PawnCharacter_C|GetLocalSounds _asvive_pawn_character) self)
    (Variables|Default|SetPlayer _asvive_pawn_character)))

(event OnComponentEndOverlap(Sphere)
  (params (OverlappedComponent :type Primitive%20Component%20Object%20Reference) (OtherActor :type Actor%20Object%20Reference) (OtherComp :type Primitive%20Component%20Object%20Reference) (OtherBodyIndex :type Integer))
  ;[1 1 1] On Begin and End Overlap
  (bind _asvive_pawn_character (Utilities|Casting|CastToVive_PawnCharacter OtherActor))
  (Utilities|Array|RemoveItem (Variables|/Game/VRExpansion/Vive/Vive_PawnCharacter.Vive_PawnCharacter_C|GetLocalSounds _asvive_pawn_character) self)
  (Variables|Default|SetPlayer 0))

(event Custom|CustomEvent
  (params (Damage :type Integer))
  ;[1 1 1] On/Off
  ;;[1 1 1] Damage
  (Variables|Default|SetDestroyed (Variables|Default|GetDestroyed)))

(event Custom|CustomEvent_1
  ;[1 1 1] On/Off
  ;;[1 1 1] Switch Interface
  (bind _isa (Utilities|FlowControl|FlipFlop) ; IsOn?
    (:A
      (if (Variables|Default|GetDestroyed)
        _))))

(event EventTick
  (params (DeltaSeconds :type Float%20%28single-precision%29))
  ;[1 1 1] Ambient Noise
  (Utilities|IsValid (Variables|Default|GetPlayer)
    (:Is%20Valid
      (if true
        (if (Variables|Default|GetDestroyed)
          (Variables|Default|SetLoudness 0.0 :!label _label)
          (elif (Variables|Default|GetIsOn)
            (Variables|Default|SetLoudness (|(pow((1-(pow(({D704A14A-4CF7-3C05-1CE9-B881DBD58D3C}/radius),4))),2)) (Variables|Default|GetDistance)))
            (Development|PrintText (Utilities|Text|FormatText "{y} distance" (Transformation|GetDistanceTo (Variables|Default|GetPlayer))) true true "(R=0.011136,G=1.000000,B=0.000000,A=1.000000)")
            (else
              (goto _label))))
        (else
          (goto _label))))))

(event EventBeginPlay
  ;[1 1 1] BeginPlay
  (bind _outattenuationsettings (Audio|Components|Audio|GetAttenuationSettingsToApply (Variables|Default|GetAudio)))
  (Variables|Default|SetDistance (.FalloffDistance (Utilities|Struct|BreakSoundAttenuationSettings _outattenuationsettings))))

(fn ConstructionScript)